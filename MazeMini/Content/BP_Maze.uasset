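; BP_Maze is a maze board actor that the player tilts through the TiltVert and TiltLR input axes.
; Each axis value, scaled by RotationSpeed, rotates BoardMesh, which is then clamped to a small angle range.
; Pitch is applied in world space and roll in local space to keep the whole board from turning.
; GetGoal exposes the CAGoal child actor cast to BP_Goal.
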(event `InputAxis|TiltVert`
  (params (AxisValue :type "Float (single-precision)"))
  (bind (_returnvalue_roll _returnvalue_pitch _returnvalue_yaw) (`KismetMathLibrary.BreakRotator` (`SceneComponent.K2_GetComponentRotation` (`self.BoardMesh`))))
  ;[1 1 1] Logic for tilting vertically (axis-wise) (pitch)
  ;;[1 1 1] Adjust board rotation base on mouse location
  (`SceneComponent.K2_AddWorldRotation` (`self.BoardMesh`) (`KismetMathLibrary.MakeRotator` 0.0 (* AxisValue (`self.RotationSpeed`))) false false)
  ;;[1 1 1] Set angle bounds so that board doesn't tilt infinitely
  (`SceneComponent.K2_SetWorldRotation` (`self.BoardMesh`) (`KismetMathLibrary.MakeRotator` _returnvalue_roll (`KismetMathLibrary.FClamp` _returnvalue_pitch -5.0 5.0) _returnvalue_yaw) false false))

(event `InputAxis|TiltLR`
  (params (AxisValue :type "Float (single-precision)"))
  (bind (_relativerotation_roll _relativerotation_pitch _relativerotation_yaw) (`KismetMathLibrary.BreakRotator` (`SceneComponent.RelativeRotation` (`self.BoardMesh`))))
  ;[1 1 1] Logic for tilting left/right (roll)
  ;;[1 1 1] Locally rotating for left and right roll so that entire board doesn't rotate upon user mouse movement
  (`SceneComponent.K2_AddLocalRotation` (`self.BoardMesh`) (`KismetMathLibrary.MakeRotator` (* AxisValue (`self.RotationSpeed`))) false false)
  ;;[1 1 1] Set angle bounds so that board doesn't tilt infinitely
  (`SceneComponent.K2_SetRelativeRotation` (`self.BoardMesh`) (`KismetMathLibrary.MakeRotator` (`KismetMathLibrary.FClamp` _relativerotation_roll -5.0 5.0) _relativerotation_pitch _relativerotation_yaw) false false))

(fn `GetGoal`
  (returns (Goal :type "/Game/BP_Goal Object Reference"))
  ;[1 1 1] Function to get goal from the child actor since return type of child actor is not the goal itself
  (return (cast `/Game/BP_Goal` (`ChildActorComponent.ChildActor` (`self.CAGoal`)) :!pure true)))

(fn `UserConstructionScript`)